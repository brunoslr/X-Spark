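; GruntCharacter is a Grunt pawn that explodes on death, hurting nearby player characters.
; On BeginPlay it runs a Possess call on GruntController, and AnyDamage subtracts incoming damage from its Health.
; At zero Health it calls DealDamageOnRadius, spawns the explosion emitter and destroys itself.
; The radial damage is hand-built, looping over all MyCharacter actors and applying flat damage to those within range.
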(event `self.ReceiveBeginPlay`
  (`Controller.Possess` (`self.GruntController`) null))

(event `self.ReceiveAnyDamage`
  (params (Damage :type "Float (single-precision)") (DamageType :type "DamageType Object Reference") (InstigatedBy :type "Controller Object Reference") (DamageCauser :type "Actor Object Reference"))
  (bind _health (`self.Health`))
  ;[1 1 1] Damage to Grunt
  (set `self.Health` (- _health Damage))
  (if (<= _health 0.0)
    (`self.DealDamageOnRadius` 150.0 50.0)
    (`GameplayStatics.SpawnEmitterAtLocation` "/Game/ParticleEffects/GruntExplode.GruntExplode" (`self.K2_GetActorLocation`))
    (`self.K2_DestroyActor`)))

(fn `DealDamageOnRadius`
  (params (Radius :type "Float (double-precision)") (Damage :type "Float (double-precision)"))
  (bind _outactors (`GameplayStatics.GetAllActorsOfClass` "/Game/Blueprints/MyCharacter.MyCharacter_C"))
  (for _array_element _outactors
    (bind _returnvalue (`self.GetDistanceTo` _array_element self))
    (if (> Radius _returnvalue)
      (`GameplayStatics.ApplyDamage` _array_element Damage null self))))

(fn `UserConstructionScript`)