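; Color-coded arc actor that projects an electricity beam onto the Mothership's shield and can be knocked out by the matching player.
; BeginPlay spawns the beam emitter at the arc mesh, and Tick keeps its target on the shield's location.
; UpdateColor sets ColorIndex and its materials, and only bullets whose PlayerIndex matches it reduce Health.
; At zero Health, ArcDown only swaps two mesh materials to glass, leaving the beam running.
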(event `self.ReceiveBeginPlay`
  (`self.SpawnElectricArcs`))

(event `SpawnElectricArcs`
  (bind _returnvalue (`SceneComponent.K2_GetComponentLocation` (`self.arc_mesh`)))
  (bind _returnvalue_2 (`GameplayStatics.SpawnEmitterAtLocation` "/Game/ParticleEffects/P_electricity_arc.P_electricity_arc" _returnvalue (struct) false))
  (set `self.ElectricArc` _returnvalue_2)
  (`ParticleSystemComponent.SetBeamSourcePoint` (`self.ElectricArc`) 0 _returnvalue 0))

(event `self.ReceiveTick`
  (params (DeltaSeconds :type "Float (single-precision)"))
  (`ParticleSystemComponent.SetBeamTargetPoint` (`self.ElectricArc`) 0 (`SceneComponent.K2_GetComponentLocation` (`/Game/Blueprints/MotherShip/MotherShip.Shield` (`self.Mothership`))) 0))

(event `self.ReceiveAnyDamage`
  (params (Damage :type "Float (single-precision)") (DamageType :type "DamageType Object Reference") (InstigatedBy :type "Controller Object Reference") (DamageCauser :type "Actor Object Reference"))
  (bind _health (`self.Health`))
  ;[1 1 1] Damage to arc
  (bind _ascharacterbullet_c (cast `/Game/Blueprints/Projectiles/CharacterBullet` DamageCauser))
  (if (== (`/Game/Blueprints/Projectiles/CharacterBullet.Player Index` _ascharacterbullet_c) (`self.ColorIndex`))
    (set `self.Health` (- _health Damage))
    (if (<= _health 0.0)
      (`self.ArcDown`))))

(fn `ArcDown`
  (bind _arc_mesh (`self.arc_mesh`))
  (`PrimitiveComponent.SetMaterial` _arc_mesh 1 "/Game/Materials/M_Glass.M_Glass")
  (`PrimitiveComponent.SetMaterial` _arc_mesh 7 "/Game/Materials/M_Glass.M_Glass"))

(fn `updateColor`
  (params (ColorIndex :type "Integer (by ref)"))
  (bind _arc_mesh (`self.arc_mesh`))
  (bind _item (`KismetArrayLibrary.Array_Get` (`self.arcMaterials`) (`self.ColorIndex`)))
  (set `self.ColorIndex` ColorIndex)
  (`PrimitiveComponent.SetMaterial` _arc_mesh 1 _item)
  (`PrimitiveComponent.SetMaterial` _arc_mesh 7 _item)
  (`PrimitiveComponent.SetMaterial` _arc_mesh 2 (`KismetArrayLibrary.Array_Get` (`self.SparkMaterials`) (`self.ColorIndex`))))

(fn `UserConstructionScript`)