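; CharacterBullet is a projectile Blueprint that damages whatever it hits and then destroys itself.
; The construction script copies FireSpeed into the projectile movement component's initial speed.
; UpdateColor maps an index to a blue, yellow, red or green Mothership material instance on the Bullet component.
; An explosion emitter spawn is left in the event graph but never runs.
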(event `self.ReceiveHit`
  (params (MyComp :type "PrimitiveComponent Object Reference") (Other :type "Actor Object Reference") (OtherComp :type "PrimitiveComponent Object Reference") (bSelfMoved :type Boolean) (HitLocation :type "Object.Vector Structure") (HitNormal :type "Object.Vector Structure") (NormalImpulse :type "Object.Vector Structure") (Hit :type "EngineTypes.HitResult Structure (by ref)"))
  (`GameplayStatics.ApplyDamage` Other 5.0 null self)
  (`self.K2_DestroyActor`))

(fn `UpdateColor`
  (params (ColorIndex :type Integer))
  (bind _bullet (`self.Bullet`))
  (switch `int` ColorIndex
    (:`0`
      (`PrimitiveComponent.SetMaterial` _bullet 0 "/Game/3DModels/mothership/mothershipMaterial_Inst_blue.mothershipMaterial_Inst_blue"))
    (:`1`
      (`PrimitiveComponent.SetMaterial` _bullet 0 "/Game/3DModels/mothership/mothershipMaterial_Inst_yellow.mothershipMaterial_Inst_yellow"))
    (:`2`
      (`PrimitiveComponent.SetMaterial` _bullet 0 "/Game/3DModels/mothership/mothershipMaterial_Inst_red.mothershipMaterial_Inst_red"))
    (:`3`
      (`PrimitiveComponent.SetMaterial` _bullet 0 "/Game/3DModels/mothership/mothershipMaterial_Inst_green.mothershipMaterial_Inst_green"))))

(fn `UserConstructionScript`
  (set `ProjectileMovementComponent.InitialSpeed` (`self.Fire Speed`) (`self.ProjectileMovement1`)))