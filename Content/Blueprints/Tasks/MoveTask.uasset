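; Behavior Tree task that glides an AI-controlled pawn toward the MoveEndLocation blackboard vector.
; Each tick it eases the pawn's location with VInterpTo and sets it directly without sweep, bypassing navigation and collision sweeps.
; It ends once the next interpolation step is small on Y and Z, ignoring X and actual distance to the target.
; Completion reports failure through FinishExecute(false).
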(event `self.ReceiveTick`
  (params (OwnerActor :type "Actor Object Reference") (DeltaSeconds :type "Float (single-precision)"))
  (bind _asaicontroller (cast `AIController` OwnerActor))
  (bind _returnvalue (`Controller.K2_GetPawn` _asaicontroller))
  (bind _returnvalue_2 (`Actor.K2_GetActorLocation` _returnvalue))
  (bind _returnvalue_3 (`KismetMathLibrary.VInterpTo` _returnvalue_2 (`BTFunctionLibrary.GetBlackboardValueAsVector` (`self.MoveEndLocation`)) DeltaSeconds 0.5))
  (`Actor.K2_SetActorLocation` _returnvalue _returnvalue_3 false)
  (bind (_returnvalue_x _returnvalue_y _returnvalue_z) (`KismetMathLibrary.BreakVector` (- _returnvalue_2 _returnvalue_3)))
  (if (and (`KismetMathLibrary.NearlyEqual_FloatFloat` (`KismetMathLibrary.Abs` _returnvalue_y) 1.0 1.0) (`KismetMathLibrary.NearlyEqual_FloatFloat` (`KismetMathLibrary.Abs` _returnvalue_z) 1.0 1.0))
    (`self.FinishExecute` false)))