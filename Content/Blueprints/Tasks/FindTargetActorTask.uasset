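; Behavior tree task that picks a random visible TargetClass actor as the AI drone's next target position.
; It line-traces on Visibility from the controlled pawn to every TargetClass actor, then filters the hit actors by that class.
; Each filtered hit overwrites the FoundPlayer blackboard bool by whether it is MyCharacter, so the last one wins.
; A random filtered actor's location is written to TargetActorPosition, using a maximum index of the array length.
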(event `self.ReceiveExecute`
  (params (OwnerActor :type "Actor Object Reference"))
  (bind _targetpointsinrange (`self.TargetPointsInRange`))
  (bind _foundplayer (`self.FoundPlayer`))
  (`KismetArrayLibrary.Array_Clear` (`self.TargetPointsInRange`))
  ;[1 1 1] Gets all target points and creates a raycast from the drone to each target point
  (bind _asaicontroller (cast `AIController` OwnerActor))
  (bind _outactors (`GameplayStatics.GetAllActorsOfClass` (`self.TargetClass`)))
  (for (_array_element _array_index) _outactors
    (bind _outhit (`KismetSystemLibrary.LineTraceSingle` (`Actor.K2_GetActorLocation` (`Controller.K2_GetPawn` _asaicontroller)) (`Actor.K2_GetActorLocation` _array_element) "TraceTypeQuery1"))
    ;[1 1 1] Inserts the objects hit by raycast into an array
    (`KismetArrayLibrary.Array_Insert` _targetpointsinrange (`.HitActor` (`GameplayStatics.BreakHitResult` _outhit)) _array_index))
  ;[1 1 1] Filters the array by Target point class type and gets a random one // Straight line of sight
  (bind _filteredarray (`KismetArrayLibrary.FilterArray` _targetpointsinrange (`self.TargetClass`)))
  (`|ExecutionSequence`
    (:`then_0`
      (for _array_element_2 _filteredarray
        (if (== (`GameplayStatics.GetObjectClass` _array_element_2) "/Game/Blueprints/MyCharacter.MyCharacter_C")
          (`BTFunctionLibrary.SetBlackboardValueAsBool` _foundplayer true)
          (else
            (`BTFunctionLibrary.SetBlackboardValueAsBool` _foundplayer)))))
    (:`then_1`
      ;[1 1 1] Set the EndLocation from the randomly picked TargetPoint
      (`BTFunctionLibrary.SetBlackboardValueAsVector` (`self.TargetActorPosition`) (`Actor.K2_GetActorLocation` (`KismetArrayLibrary.Array_Get` _filteredarray (`KismetMathLibrary.RandomIntegerInRange` 0 (`KismetArrayLibrary.Array_Length` _filteredarray)))))
      (`self.FinishExecute` true))))