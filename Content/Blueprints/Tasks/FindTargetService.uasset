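; A behavior tree service for grunt AI that picks the nearest pawn to follow.
; Each tick it sphere-traces from the controlled pawn toward every actor of the target class, using the search radius as trace radius and initial distance limit.
; The closest pawn hit, not filtered by class, is written to the blackboard as follow target and location, which are never cleared here.
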(event `self.ReceiveTick`
  (params (OwnerActor :type "Actor Object Reference") (DeltaSeconds :type "Float (single-precision)"))
  (set `self.ShortestDistance` (`self.SearchRadius`))
  (bind _asgruntcontroller_c (cast `/Game/Blueprints/Grunt/GruntController` OwnerActor))
  (set `self.Grunt_controller` _asgruntcontroller_c)
  (bind _outactors (`GameplayStatics.GetAllActorsOfClass` (`self.TargetClass`)))
  (for _array_element _outactors
    (bind _outhits (`KismetSystemLibrary.SphereTraceMultiForObjects` (`Actor.K2_GetActorLocation` (`Controller.K2_GetPawn` _asgruntcontroller_c)) (`Actor.K2_GetActorLocation` _array_element) (`self.SearchRadius`) (`|MakeArray` "ObjectTypeQuery3" :!type "EngineTypes.EObjectTypeQuery Enum")))
    (for _array_element_2 _outhits
      (bind (_location _normal _impactpoint _impactnormal _physmat _hitactor) (`GameplayStatics.BreakHitResult` _array_element_2))
      (bind _returnvalue (`Actor.GetDistanceTo` _hitactor (`Controller.K2_GetPawn` (`self.Grunt_controller`))))
      (if (> (`self.ShortestDistance`) _returnvalue)
        (set `self.ShortestDistance` _returnvalue)
        (`BTFunctionLibrary.SetBlackboardValueAsObject` (`self.TargetToFollow`) _hitactor)
        (`BTFunctionLibrary.SetBlackboardValueAsVector` (`self.TargetLocation`) (`Actor.K2_GetActorLocation` _hitactor))))))