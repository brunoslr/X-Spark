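; Behavior Tree task that deals area damage around an AI-controlled pawn.
; On execute, it gets every MyCharacter in the level and applies Damage to those closer than Radius, with the pawn as damage causer.
; It uses a plain distance check with no overlap query or line-of-sight test.
; The task finishes successfully after the loop, but never calls FinishExecute if the owner is not an AIController.
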(event `self.ReceiveExecute`
  (params (OwnerActor :type "Actor Object Reference"))
  (bind _asaicontroller (cast `AIController` OwnerActor))
  (bind _outactors (`GameplayStatics.GetAllActorsOfClass` "/Game/Blueprints/MyCharacter.MyCharacter_C"))
  (for _array_element _outactors
    (bind _returnvalue (`Controller.K2_GetPawn` _asaicontroller))
    (bind _returnvalue_2 (`Actor.GetDistanceTo` _returnvalue _array_element))
    (if (> (`self.Radius`) _returnvalue_2)
      (`GameplayStatics.ApplyDamage` _array_element (`self.Damage`) null _returnvalue)))
  (`self.FinishExecute` true))