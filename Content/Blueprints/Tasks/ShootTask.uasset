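; Behavior tree task that makes an AI-controlled pawn fire at a target.
; When the FoundPlayer blackboard flag is set, it spawns a half-scale EnemyBullet at the pawn's location, rotated toward the ShootTarget blackboard vector with a set fire speed.
; The task always finishes successfully, whether or not it fires.
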(event `self.ReceiveExecute`
  (params (OwnerActor :type "Actor Object Reference"))
  (if (`BTFunctionLibrary.GetBlackboardValueAsBool` (`self.FoundPlayer`))
    (`self.AIFire` OwnerActor)
    (`self.FinishExecute` true)
    (else
      (`self.FinishExecute` true))))

(fn `AIFire`
  (params (OwnerActor :type "Actor Object Reference"))
  (bind _asaicontroller (cast `AIController` OwnerActor))
  (bind _returnvalue (`Actor.K2_GetActorLocation` (`Controller.K2_GetPawn` _asaicontroller)))
  (`|SpawnActorFromClass` "/Game/Blueprints/Projectiles/EnemyBullet.EnemyBullet_C" (`KismetMathLibrary.MakeTransform` _returnvalue (`KismetMathLibrary.FindLookAtRotation` _returnvalue (`BTFunctionLibrary.GetBlackboardValueAsVector` (`self.ShootTarget`))) (0.5 0.5 0.5)) false 1500.0))