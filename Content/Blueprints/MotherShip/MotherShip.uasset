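; Mothership boss that spawns drones and grunts on timers and pauses its timeline-driven movement to fire a sweeping line-trace beam laser at players.
; Only bullets whose player index matches its color index damage it; the color re-rolls randomly while unshielded and not firing.
; Two Arc actors, given colors different from the ship's, hold up its shield.
; Destroying both enables collision until a delay restores and recolors them.
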(event `self.ReceiveBeginPlay`
  ;[1 1 1] Ship Movement Speed / Laser Play Rate / Updating Color Index / Getting Arcs
  (`|ExecutionSequence`
    (:`then_0`
      (`TimelineComponent.SetPlayRate` (`self.ShipMotion`) (/ 1.0 (`self.Travel Time `)))
      (set `self.Test End Location` false))
    (:`then_1`
      (`TimelineComponent.SetPlayRate` (`self.LaserDirectionTurn`) (/ 1.0 5.0)))
    (:`then_2`
      (`self.UpdateColorIndex` (`KismetMathLibrary.RandomInteger` 4)))
    (:`then_3`
      (bind _outactors (`GameplayStatics.GetAllActorsOfClass` "/Game/Blueprints/Arc/arcBlueprint.ArcBlueprint_C"))
      (for (_array_element _array_index) _outactors
        (bind _asarcblueprint_c (cast `/Game/Blueprints/Arc/arcBlueprint` _array_element))
        (`KismetArrayLibrary.Array_Insert` (`self.Arcs`) _asarcblueprint_c _array_index))
      (`self.ArcShipColorCheck`))))

(event `self.ReceiveAnyDamage`
  (params (Damage :type "Float (single-precision)") (DamageType :type "DamageType Object Reference") (InstigatedBy :type "Controller Object Reference") (DamageCauser :type "Actor Object Reference"))
  (bind _health (`self.Health`))
  ;[1 1 1] Damage to Spaceship
  (bind _ascharacterbullet_c (cast `/Game/Blueprints/Projectiles/CharacterBullet` DamageCauser))
  (if (== (`/Game/Blueprints/Projectiles/CharacterBullet.Player Index` _ascharacterbullet_c) (`self.MothershipColorIndex`))
    (`KismetSystemLibrary.PrintString` (`KismetStringLibrary.Conv_DoubleToString` _health))
    (set `self.Health` (- _health Damage))
    (if (<= _health 0.0)
      (`GameplayStatics.SpawnEmitterAtLocation` "/Game/ParticleEffects/P_Explosion2.P_Explosion2" (`SceneComponent.K2_GetComponentLocation` (`self.MotherShip`)))
      (`self.K2_DestroyActor`))))

(event `StartLaser`
  (bind _laserpoint (`self.LaserPoint`))
  ;[1 1 1] Fire Laser
  (set `self.FiringLaser` true)
  (bind _returnvalue (`GameplayStatics.SpawnEmitterAtLocation` "/Game/ParticleEffects/LaserBeamParticle.LaserBeamParticle" (`SceneComponent.K2_GetComponentLocation` (`self.LaserPoint`)) (struct) false))
  (set `self.LaserParticle` _returnvalue)
  (bind (_direction _newtrack_1) (`Timeline|LaserDirectionTurn` :`NewTime` 1.0 :!via `PlayFromStart`)
    (:`Update`
      (`SceneComponent.SetWorldRotation` _laserpoint (`KismetMathLibrary.RLerp` (`self.RightPosition`) (`self.LeftPosition`) _newtrack_1) false)
      (`self.FireLaser`))
    (:`Finished`
      (`ActorComponent.K2_DestroyComponent` (`self.LaserParticle`))
      (set `self.FiringLaser` false)
      (`SceneComponent.SetWorldRotation` :`self` _laserpoint)
      (`self.MoveShip`)
      (set `self.ElapsedTime` 0.0)
      (set `self.DroneSpawnTimer` 0.0)
      (set `self.GruntSpawnTimer` 0.0))))

(event `MoveShip`
  ;[1 1 1] Movement / Starting Laser
  (bind (_direction _lerp_alpha) (`Timeline|ShipMotion` :!label _label)
    (:`Update`
      (bind _returnvalue (`KismetMathLibrary.VLerp` (0.0 0.0 0.0) (`self.End Location`) _lerp_alpha))
      (`SceneComponent.SetRelativeLocation` (`self.MotherShip`) _returnvalue false)
      (`SceneComponent.SetRelativeLocation` (`self.Shield`) (+ _returnvalue (0.0 0.0 60.0)) false)
      (if (>= (`self.ElapsedTime`) 12.0)
        (`self.StopShip`)
        (`self.StartLaser`)
        (set `self.ElapsedTime` 0.0)))))

(event `self.ReceiveTick`
  (params (DeltaSeconds :type "Float (single-precision)"))
  (bind _bvisible (`SceneComponent.bVisible` (`self.Shield`)))
  (`|ExecutionSequence`
    (:`then_0`
      ;[1 1 1] Change Color / Set the time to change color here
      (set `self.DeltaSeconds` DeltaSeconds)
      (set `self.ElapsedTime` (+ DeltaSeconds (`self.ElapsedTime`)))
      (set `self.DroneSpawnTimer` (+ DeltaSeconds (`self.DroneSpawnTimer`)))
      (set `self.GruntSpawnTimer` (+ DeltaSeconds (`self.GruntSpawnTimer`)))
      (if (not (or (`self.FiringLaser`) _bvisible))
        (`KismetSystemLibrary.Delay` 4.0)
        (if (not _bvisible)
          (`self.UpdateColorIndex` (`KismetMathLibrary.RandomInteger` 4)))))
    (:`then_1`
      ;[1 1 1] GruntSpawn
      (if (and (>= (`self.GruntSpawnTimer`) 4.5) (== (`self.FiringLaser`) false))
        (`self.SpawnGrunt`)
        (set `self.GruntSpawnTimer` (`KismetMathLibrary.RandomFloatInRange` 0.0 3.5))))
    (:`then_2`
      ;[1 1 1] DroneSpawn
      (if (and (>= (`self.DroneSpawnTimer`) 3.5) (== (`self.FiringLaser`) false))
        (`self.SpawnDrones`)
        (set `self.DroneSpawnTimer` 0.0)))
    (:`then_3`
      (`self.ArcHealthCheck`)
      (`self.ShieldCollision`)
      (if (`self.ShieldState`)
        (`KismetSystemLibrary.Delay` 10.0)
        (for _array_element (`self.Arcs`)
          (set `/Game/Blueprints/Arc/arcBlueprint.Health` 25.0 _array_element)
          (`/Game/Blueprints/Arc/arcBlueprint.SpawnElectricArcs` _array_element))
        (`self.ArcShipColorCheck`)))))

(event `StopShip`
  ;[1 1 1] Movement / Starting Laser
  (goto _label :!via `Stop`))

(fn `ArcHealthCheck`
  (bind _arcs (`self.Arcs`))
  (bind _item (`KismetArrayLibrary.Array_Get` _arcs 1))
  (bind _item_2 (`KismetArrayLibrary.Array_Get` _arcs))
  (bind _returnvalue (<= (`/Game/Blueprints/Arc/arcBlueprint.Health` _item) 0.0))
  (bind _returnvalue_2 (<= (`/Game/Blueprints/Arc/arcBlueprint.Health` _item_2) 0.0))
  (`|ExecutionSequence`
    (:`then_0`
      (if _returnvalue_2
        (`ActorComponent.K2_DestroyComponent` (`/Game/Blueprints/Arc/arcBlueprint.ElectricArc` _item_2))))
    (:`then_1`
      (if _returnvalue
        (`ActorComponent.K2_DestroyComponent` (`/Game/Blueprints/Arc/arcBlueprint.ElectricArc` _item))))
    (:`then_2`
      (if (and _returnvalue_2 _returnvalue)
        (set `self.BothArcDown` true)
        (else
          (set `self.BothArcDown` false))))))

(fn `ArcShipColorCheck`
  (bind _arc2colorindex (`self.Arc2ColorIndex`))
  (bind _arcs (`self.Arcs`))
  (bind _item (`KismetArrayLibrary.Array_Get` _arcs 1))
  (set `self.Arc1ColorIndex` (mod (+ (`self.MothershipColorIndex`) (`KismetMathLibrary.RandomIntegerInRange` 1 3)) 4))
  (`/Game/Blueprints/Arc/arcBlueprint.updateColor` (`KismetArrayLibrary.Array_Get` _arcs) (`self.Arc1ColorIndex`))
  (set `self.Arc2ColorIndex` (mod (+ (`self.MothershipColorIndex`) 1) 4))
  (if (== (`self.Arc2ColorIndex`) (`self.Arc1ColorIndex`))
    (set `self.Arc2ColorIndex` (mod (+ (`self.Arc2ColorIndex`) 1) 4))
    (`/Game/Blueprints/Arc/arcBlueprint.updateColor` _item _arc2colorindex)
    (else
      (`/Game/Blueprints/Arc/arcBlueprint.updateColor` _item _arc2colorindex))))

(fn `FireLaser`
  (bind _laserparticle (`self.LaserParticle`))
  (bind _laserpoint (`self.LaserPoint`))
  (bind _returnvalue (`SceneComponent.K2_GetComponentLocation` _laserpoint))
  (bind _outhit (`KismetSystemLibrary.LineTraceSingle` _returnvalue (+ _returnvalue (* (`SceneComponent.GetUpVector` _laserpoint) -10000.0)) "TraceTypeQuery2" true))
  (`ParticleSystemComponent.SetBeamSourcePoint` _laserparticle 0 (`SceneComponent.K2_GetComponentLocation` (`self.LaserPoint`)) 0)
  (bind (_location _normal _impactpoint _impactnormal _physmat _hitactor) (`GameplayStatics.BreakHitResult` _outhit))
  (`ParticleSystemComponent.SetBeamTargetPoint` _laserparticle 0 _location 0)
  (bind _asmycharacter_c (cast `/Game/Blueprints/MyCharacter` _hitactor))
  (`GameplayStatics.ApplyDamage` _asmycharacter_c 100.0))

(fn `ShieldandArc`)

(fn `ShieldCollision`
  (if (`self.BothArcDown`)
    (`self.SetActorEnableCollision` true)
    (`SceneComponent.SetVisibility` (`self.Shield`) false false)
    (set `self.ShieldState` true)
    (else
      (`self.SetActorEnableCollision` false)
      (`SceneComponent.SetVisibility` (`self.Shield`) true false)
      (set `self.ShieldState` false))))

(fn `SpawnDrones`
  (`AIBlueprintHelperLibrary.SpawnAIFromClass` "/Game/Blueprints/Drone/AIDroneCharacter.AIDroneCharacter_C" "/Game/Blueprints/Drone/AIDroneBehaviorTree.AIDroneBehaviorTree" (`SceneComponent.K2_GetComponentLocation` (`self.LaserPoint`))))

(fn `SpawnElectricArcs`)

(fn `SpawnGrunt`
  (`AIBlueprintHelperLibrary.SpawnAIFromClass` "/Game/Blueprints/Grunt/GruntCharacter.GruntCharacter_C" "/Game/Blueprints/Grunt/GruntBT.GruntBT" (`SceneComponent.K2_GetComponentLocation` (`self.LaserPoint`))))

(fn `UpdateColorIndex`
  (params (ColorIndex :type Integer))
  (bind _mothership (`self.MotherShip`))
  (bind _item (`KismetArrayLibrary.Array_Get` (`self.Materials`) (`self.MothershipColorIndex`)))
  (set `self.MothershipColorIndex` ColorIndex)
  (`PrimitiveComponent.SetMaterial` _mothership 0 _item)
  (`PrimitiveComponent.SetMaterial` _mothership 3 _item))

(fn `UserConstructionScript`
  (`SceneComponent.SetRelativeLocation` (`self.MotherShip`) (`KismetMathLibrary.SelectVector` (`self.End Location`) (0.0 0.0 0.0) (`self.Test End Location`)) false))