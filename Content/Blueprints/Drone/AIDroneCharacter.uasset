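; AI drone character that takes damage and is destroyed when its health runs out.
; On BeginPlay it calls Possess on its drone controller.
; AnyDamage activates a Fire effect at low health, testing health before subtracting the hit, then destroys the actor at zero or below.
; SetSpeed and the construction script are empty.
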(event `self.ReceiveBeginPlay`
  (`Controller.Possess` (`self.DroneController`) null))

(event `self.ReceiveAnyDamage`
  (params (Damage :type "Float (single-precision)") (DamageType :type "DamageType Object Reference") (InstigatedBy :type "Controller Object Reference") (DamageCauser :type "Actor Object Reference"))
  (bind _health (`self.Health`))
  ;[1 1 1] Damage to Drone
  (`|ExecutionSequence`
    (:`then_0`
      (if (<= _health 20.0)
        (`ActorComponent.Activate` (`self.Fire`) false)))
    (:`then_1`
      (set `self.Health` (- _health Damage))
      (if (<= _health 0.0)
        (`self.K2_DestroyActor`)))))

(fn `SetSpeed`
  (params (Speed :type "Float (double-precision)")))

(fn `UserConstructionScript`)